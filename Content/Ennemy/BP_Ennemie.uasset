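; Enemy Blueprint that turns its mesh to face the player, attacks at close range and takes damage until it dies.
; Detection and attack sphere overlaps, unfiltered by actor, set aggro and range flags that Tick reads to rotate and trigger the attack montage with a cooldown.
; The Attack event receives damage despite its name, playing a hit montage and, at zero health, enabling mesh physics and disabling hitbox collision.
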(event `self.Detection Sphere.OnComponentBeginOverlap`
  (params (OverlappedComponent :type "PrimitiveComponent Object Reference") (OtherActor :type "Actor Object Reference") (OtherComp :type "PrimitiveComponent Object Reference") (OtherBodyIndex :type Integer) (bFromSweep :type Boolean) (SweepResult :type "HitResult Structure (by ref)"))
  (set `self.IsAgro` true)
  (`KismetSystemLibrary.PrintString` "En garde"))

(event `self.ReceiveTick`
  (params (DeltaSeconds :type "Float (single-precision)"))
  (bind (_returnvalue_roll _returnvalue_pitch _returnvalue_yaw) (`KismetMathLibrary.BreakRotator` (`KismetMathLibrary.FindLookAtRotation` (`SceneComponent.K2_GetComponentLocation` (`self.SkeletalMesh`)) (`self.K2_GetActorLocation` (`GameplayStatics.GetPlayerCharacter` 0)))))
  (if (`self.IsAgro`)
    (`SceneComponent.K2_SetWorldRotation` (`self.SkeletalMesh`) (`KismetMathLibrary.MakeRotator` 0.0 0.0 (+ _returnvalue_yaw -90.0)) false false)
    (if (and (`self.AttackRange`) (`self.CanAttack`))
      (`self.Attack Event`))))

(event `self.Detection Sphere.OnComponentEndOverlap`
  (params (OverlappedComponent :type "PrimitiveComponent Object Reference") (OtherActor :type "Actor Object Reference") (OtherComp :type "PrimitiveComponent Object Reference") (OtherBodyIndex :type Integer))
  (set `self.IsAgro` false)
  (`KismetSystemLibrary.PrintString` "Repos"))

(event `Attack Event`
  (set `self.CanAttack` false)
  (`|PlayMontage` (`self.SkeletalMesh`) "/Game/Ennemy/Animations/Attack.Attack"
    (:`OnCompleted`
      _)
    (:`OnInterrupted`
      _))
  (`KismetSystemLibrary.Delay` 2.0)
  (set `self.CanAttack` true))

(event `self.Attack Radius.OnComponentBeginOverlap`
  (params (OverlappedComponent :type "PrimitiveComponent Object Reference") (OtherActor :type "Actor Object Reference") (OtherComp :type "PrimitiveComponent Object Reference") (OtherBodyIndex :type Integer) (bFromSweep :type Boolean) (SweepResult :type "HitResult Structure (by ref)"))
  (set `self.AttackRange` true))

(event `Die Event`
  (`PrimitiveComponent.SetSimulatePhysics` (`self.SkeletalMesh`) true)
  (`PrimitiveComponent.SetCollisionEnabled` (`self.Hitbox`) "NoCollision"))

(event `self.Attack Radius.OnComponentEndOverlap`
  (params (OverlappedComponent :type "PrimitiveComponent Object Reference") (OtherActor :type "Actor Object Reference") (OtherComp :type "PrimitiveComponent Object Reference") (OtherBodyIndex :type Integer))
  (set `self.AttackRange` false))

(event `/Game/ThirdPerson/BPI_Attack.Attack`
  (params (DamageQuantity :type "Float (double-precision)"))
  ;[1 1 1] Take damage
  (`KismetSystemLibrary.PrintString` "Aie")
  (bind _output_get (set `self.Health` (`KismetMathLibrary.FClamp` (- (`self.Health`) DamageQuantity) 0.0 100.0)))
  (`KismetSystemLibrary.PrintString` (`KismetStringLibrary.Conv_DoubleToString` _output_get))
  (`|PlayMontage` (`self.SkeletalMesh`) "/Game/Ennemy/Animations/TakingDamage.TakingDamage"
    (:`then`
      (if (== (`self.Health`) 0.0)
        (`self.Die Event`)))))

(fn `UserConstructionScript`)